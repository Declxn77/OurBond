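; FrontDoor_BP is a front door that toggles open and closed each time its OpenDoor event fires.
; A closed-state flag decides whether to play the OpenDoorTL timeline forward or in reverse, along with an opening or closing sound.
; The timeline's alpha drives a lerp on the Door component's relative yaw, swinging it through a quarter turn.
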(event Custom|OpenDoor
  (if (Variables|Default|GetIsDoorClosed)
    (Variables|Default|SetIsDoorClosed false)
    (Audio|PlaySoundatLocation "/Game/Audio/Door/431117__inspectorj__door-front-opening-a.431117__inspectorj__door-front-opening-a" "0, 0, 0" "0, 0, 0" 1.0 1.0 0.0 0 0 0)
    (bind _alpha (Timeline|OpenDoorTL Play)
      (:Update
        (Transformation|SetRelativeRotation (Variables|Default|GetDoor) (Math|Rotator|MakeRotator 0.0 0.0 (Math|Float|Lerp 0.0 -9e+01 _alpha)) false false)))
    (else
      (Variables|Default|SetIsDoorClosed true)
      (Audio|PlaySoundatLocation "/Game/Audio/Door/431118__inspectorj__door-front-closing-a.431118__inspectorj__door-front-closing-a" "0, 0, 0" "0, 0, 0" 1.0 1.0 0.0 0 0 0)
      (Timeline|OpenDoorTL Reverse))))

(fn ConstructionScript)
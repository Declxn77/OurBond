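; Subtitle manager actor that steps through narration lines stored in a Data Table and displays them on an InspectUI widget.
; ShowLine forwards to ShowNextLine, which restarts at the first row when FirstLine is set, displays that row's LineToShow and advances CurrentRow.
; ClearSubtitles blanks the displayed line.
; The widget creation nodes are disconnected, so nothing here sets SubtitlesWidgetREF at runtime.
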(event Custom|ClearSubtitles
  (Default|DisplayLine (Variables|Default|GetSubtitlesWidgetREF)))

(event Custom|ShowNextLine
  (params (FirstLine :type Boolean) (NarrationList :type Data%20Table%20Object%20Reference))
  (Variables|Default|SetCurrentNarration%20List NarrationList)
  (if FirstLine
    (Variables|Default|SetCurrentRow 0)
    (bind _outrownames (DataTable|GetDataTableRowNames (Variables|Default|GetCurrentNarration%20List)))
    (bind _returnvalue (Utilities|GetDataTableRow (Variables|Default|GetCurrentNarration%20List) (Utilities|Array|Get(acopy) _outrownames (Variables|Default|GetCurrentRow)))
      (:then
        (Default|DisplayLine (Variables|Default|GetSubtitlesWidgetREF) (.LineToShow (Utilities|Struct|BreakSubtitlesStruct _returnvalue)))
        (Variables|Default|SetCurrentRow (+ (Variables|Default|GetCurrentRow) 1))))
    (else
      (bind _outrownames_2 (DataTable|GetDataTableRowNames (Variables|Default|GetCurrentNarration%20List)))
      (bind _returnvalue_2 (Utilities|GetDataTableRow (Variables|Default|GetCurrentNarration%20List) (Utilities|Array|Get(acopy) _outrownames_2 (Variables|Default|GetCurrentRow)))
        (:then
          (Default|DisplayLine (Variables|Default|GetSubtitlesWidgetREF) (.LineToShow (Utilities|Struct|BreakSubtitlesStruct _returnvalue_2)))
          (Variables|Default|SetCurrentRow (+ (Variables|Default|GetCurrentRow) 1)))))))

(event Collision|EventActorBeginOverlap
  (params (OtherActor :type Actor%20Object%20Reference)))

(event EventTick
  (params (DeltaSeconds :type Float%20%28single-precision%29)))

(fn ConstructionScript)

(fn ShowLine
  (params (First%20Line :type Boolean) (NarrationList :type Data%20Table%20Object%20Reference))
  (CallFunction|ShowNextLine First%20Line NarrationList))
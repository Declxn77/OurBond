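; TestSound is an interactable test Blueprint that plays a sound and briefly freezes the player's movement.
; Its Interact event passes through a DoOnce, prints a string, ignores move input on the first player controller and plays the sound at world origin.
; A two-second timer then fires a custom event that restores movement input.
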(event Custom|CustomEvent
  (Input|SetIgnoreMoveInput (Game|GetPlayerController 0) false))

(event EventBeginPlay)

(event Collision|EventActorBeginOverlap
  (params (OtherActor :type Actor%20Object%20Reference)))

(event EventTick
  (params (DeltaSeconds :type Float%20%28single-precision%29)))

(event EventInteract
  (params (Player :type First%20Person%20Character%20Object%20Reference))
  (Utilities|FlowControl|DoOnce false
    (:Completed
      (Development|PrintString (Variables|Default|GetIn%20String))
      (Input|SetIgnoreMoveInput (Game|GetPlayerController 0) true)
      (Audio|PlaySoundatLocation (Variables|Default|GetSound) "0, 0, 0" "0, 0, 0" 1.0 1.0 0.0 0 0 0)
      (Utilities|Time|SetTimerbyEvent (delegate Custom|CustomEvent) 2.0))))

(fn ConstructionScript)
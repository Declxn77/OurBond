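; WallButton is an interactive wall switch that toggles the lights in the level when the player presses E nearby.
; Its box collision enables input while a FirstPersonCharacter overlaps it and disables input when that character leaves.
; Each press flips its own IsOn flag, then finds every LightButton actor with GetAllActorsOfClass and calls SwitchLight on each, without passing that flag.
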(event OnComponentBeginOverlap(BoxCollision)
  (params (OverlappedComponent :type Primitive%20Component%20Object%20Reference) (OtherActor :type Actor%20Object%20Reference) (OtherComp :type Primitive%20Component%20Object%20Reference) (OtherBodyIndex :type Integer) (bFromSweep :type Boolean) (SweepResult :type Hit%20Result%20Structure%20%28by%20ref%29))
  (Utilities|Casting|CastToFirstPersonCharacter OtherActor)
  (Input|EnableInput (Game|GetPlayerController 0)))

(event OnComponentEndOverlap(BoxCollision)
  (params (OverlappedComponent :type Primitive%20Component%20Object%20Reference) (OtherActor :type Actor%20Object%20Reference) (OtherComp :type Primitive%20Component%20Object%20Reference) (OtherBodyIndex :type Integer))
  (Utilities|Casting|CastToFirstPersonCharacter OtherActor)
  (Input|DisableInput (Game|GetPlayerController 0)))

(event Input|KeyboardEvents|E
  (params (Key :type Key%20Structure :default "None"))
  (:Pressed
    (Variables|Default|SetIsOn (not (Variables|Default|GetIsOn)))
    (bind _outactors (Actor|GetAllActorsOfClass "/Game/Blueprints/LightSwitch/LightButton.LightButton_C"))
    (for _array_element _outactors
      (Default|SwitchLight _array_element))))

(fn ConstructionScript)
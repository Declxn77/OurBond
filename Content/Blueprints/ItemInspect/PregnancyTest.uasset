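; Inspectable pregnancy test memory item that shows a prompt on overlap and, on interact, moves to the camera with an item UI and depth-of-field blur.
; Input rotates and zooms it; Interact returns it to its original transform.
; First pickup plays audio and decrements the game mode's MemoriesLeft.
; Tick dot-tests InspectionVector against camera forward to trigger a second clip once that side faces the player, with timers gating input during audio.
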(event OnComponentBeginOverlap(Sphere)
  (params (OverlappedComponent :type Primitive%20Component%20Object%20Reference) (OtherActor :type Actor%20Object%20Reference) (OtherComp :type Primitive%20Component%20Object%20Reference) (OtherBodyIndex :type Integer) (bFromSweep :type Boolean) (SweepResult :type Hit%20Result%20Structure%20%28by%20ref%29))
  (bind _widget (Variables|Default|GetWidget))
  (Utilities|Casting|CastToFirstPersonCharacter OtherActor)
  (bind _returnvalue (UserInterface|CreateWidget "/Game/Blueprints/ItemInspect/InspectionHUD.InspectionHUD_C"))
  (bind _output_get (Variables|Default|SetInteractionWidget _returnvalue))
  (UserInterface|SetWidget _widget _output_get)
  (Rendering|SetVisibility _widget true false)
  (Rendering|Material|SetScalarParameterValueonMaterials (Variables|Default|GetStaticMesh) "Selected" 1.0))

(event OnComponentEndOverlap(Sphere)
  (params (OverlappedComponent :type Primitive%20Component%20Object%20Reference) (OtherActor :type Actor%20Object%20Reference) (OtherComp :type Primitive%20Component%20Object%20Reference) (OtherBodyIndex :type Integer))
  (Utilities|Casting|CastToFirstPersonCharacter OtherActor)
  (Widget|RemovefromParent (Variables|Default|GetInteractionWidget))
  (Rendering|SetVisibility (Variables|Default|GetWidget) false false)
  (Rendering|Material|SetScalarParameterValueonMaterials (Variables|Default|GetStaticMesh) "Selected" 1.0))

(event Custom|ClearSubtitles
  (Default|DisplayLine (Variables|Default|GetInspectUI)))

(event Custom|CustomEvent_2
  (Input|EnableInput (Game|GetPlayerController 0))
  (Variables|Default|SetSecondPlayed true))

(event Custom|CustomEvent
  (Input|EnableInput (Game|GetPlayerController 0))
  (Variables|Default|SetPlayed true))

(event Custom|CustomEvent_1
  (Input|EnableInput (Game|GetPlayerController 0)))

(event EventTick
  (params (DeltaSeconds :type Float%20%28single-precision%29))
  (bind _player (Variables|Default|GetPlayer)
    (:then
      (if (<= (Math|Vector|DotProduct (Math|Vector|RotateVector (Variables|Default|GetInspectionVector) (Transformation|GetWorldRotation (Variables|Default|GetStaticMesh))) (Math|Vector|GetForwardVector (Variables|/Game/FirstPersonBP/Blueprints/FirstPersonCharacter.FirstPersonCharacter_C|GetFirstPersonCamera _player))) -0.7)
        (if (Variables|Default|GetSecondPlayed)
          (Input|EnableInput (Game|GetPlayerController 0))
          (else
            (Utilities|FlowControl|DoOnce false
              (:Completed
                (Input|DisableInput (Game|GetPlayerController 0))
                (Audio|PlaySoundatLocation (Variables|Default|GetSoundClip) "0, 0, 0" "0, 0, 0" 1.0 1.0 0.0 0 0 0)
                (Utilities|Time|SetTimerbyEvent (delegate Custom|CustomEvent_2) (Variables|Default|GetAudioDelayOnVector))))))))
    (:else)))

(event EventCanRecieveTrace
  (params (CanInteract :type Boolean)))

(event EventInteract
  (params (Player :type First%20Person%20Character%20Object%20Reference))
  (Variables|Default|SetPlayer Player)
  (Collision|SetActorEnableCollision false)
  (Collision|SetCollisionProfileName (Variables|Default|GetSphere) "NoCollision" true :!class /Script/Engine.PrimitiveComponent)
  (Transformation|AttachComponentToComponent (Variables|/Script/Engine.PlayerCameraManager|GetTransformComponent (Game|GetPlayerCameraManager 0)) "None" "KeepWorld" "KeepWorld" "KeepWorld" true)
  (bind _returnvalue (UserInterface|CreateWidget "/Game/Blueprints/ItemInspect/InspectUI.InspectUI_C" 0 (Variables|Default|GetItemName) (Variables|Default|GetItemDescription)))
  (bind _output_get (Variables|Default|SetInspectUI _returnvalue))
  (UserInterface|Viewport|AddtoViewport _output_get 0)
  (CallFunction|ClearSubtitles)
  (Components|MoveComponentTo (Variables|Default|GetStaticMesh) (Variables|Default|GetTarget%20Relative%20Location) (Variables|Default|GetTarget%20Relative%20Rotation) false false 0.2 false)
  (CallFunction|ToggleDOF true)
  (Rendering|Material|SetScalarParameterValueonMaterials (Variables|Default|GetStaticMesh) "Selected" 0.0)
  (if (Variables|Default|GetPlayed)
    (Input|EnableInput (Game|GetPlayerController 0))
    (else
      (Input|DisableInput (Variables|Default|GetPlayer) (Game|GetPlayerController 0))
      (Audio|PlaySoundatLocation (Variables|Default|GetPickupClip) "0, 0, 0" "0, 0, 0" 1.0 1.0 0.0 0 0 0)
      (Utilities|Time|SetTimerbyEvent (delegate Custom|CustomEvent) (Variables|Default|GetAudioDelayOnpickup))
      (bind _asfirst_person_game_mode (Utilities|Casting|CastToFirstPersonGameMode (Game|GetGameMode)))
      (bind _result (Math|Integer|DecrementInt (Variables|/Game/FirstPersonBP/Blueprints/FirstPersonGameMode.FirstPersonGameMode_C|GetMemoriesLeft _asfirst_person_game_mode))
        (:%20%20
          (Variables|/Game/FirstPersonBP/Blueprints/FirstPersonGameMode.FirstPersonGameMode_C|SetMemoriesLeft _asfirst_person_game_mode _result))))))

(event EventBeginPlay
  (Rendering|Material|SetScalarParameterValueonMaterials (Variables|Default|GetStaticMesh) "Selected" 1.0)
  (Variables|Default|SetTransform (Transformation|GetActorTransform)))

(event Input|ActionEvents|InputActionInteract
  (params (Key :type Key%20Structure :default "None"))
  (bind _returnvalue (Game|GetPlayerController 0))
  (bind _transform (Variables|Default|GetTransform))
  (:Pressed
    (Transformation|DetachFromActor "KeepWorld" "KeepWorld" "KeepWorld")
    (Widget|RemovefromParent (Variables|Default|GetInspectUI))
    (Variables|Default|SetInspectUI 0)
    (Components|MoveComponentTo (Variables|Default|GetStaticMesh) (.location _transform) (.rotation _transform) false false 0.2 false)
    (Collision|SetActorEnableCollision true)
    (Collision|SetCollisionProfileName (Variables|Default|GetSphere) "OverlapAllDynamic" true :!class /Script/Engine.PrimitiveComponent)
    (Input|DisableInput _returnvalue)
    (Input|EnableInput (Variables|Default|GetPlayer) _returnvalue)
    (CallFunction|ToggleDOF false)
    (Variables|Default|SetPlayer 0)))

(event Input|AxisEvents|InputAxisMoveForward
  (params (AxisValue :type Float%20%28single-precision%29))
  (if (!= AxisValue 0.0)
    (Transformation|SetActorRotation (Math|Rotator|CombineRotators (Transformation|GetActorRotation) (Math|Rotator|MakeRotator 0.0 (* AxisValue -1.0) 0.0)))))

(event Input|AxisEvents|InputAxisMoveRight
  (params (AxisValue :type Float%20%28single-precision%29))
  (if (!= AxisValue 0.0)
    (Transformation|SetActorRotation (Math|Rotator|CombineRotators (Transformation|GetActorRotation) (Math|Rotator|MakeRotator 0.0 0.0 (* AxisValue -1.0))))))

(event Input|MouseEvents|MouseX
  (params (AxisValue :type Float%20%28single-precision%29))
  (if (Variables|Default|GetCanRotate)
    (Transformation|SetActorRotation (Math|Rotator|CombineRotators (Transformation|GetActorRotation) (Math|Rotator|MakeRotator 0.0 0.0 (* AxisValue -2.0))))))

(event Input|MouseEvents|MouseY
  (params (AxisValue :type Float%20%28single-precision%29))
  (if (Variables|Default|GetCanRotate)
    (Transformation|SetActorRotation (Math|Rotator|CombineRotators (Transformation|GetActorRotation) (Math|Rotator|MakeRotator 0.0 (* AxisValue 2.0) 0.0)))))

(event Input|MouseEvents|LeftMouseButton
  (params (Key :type Key%20Structure :default "None"))
  (:Pressed
    (Variables|Default|SetCanRotate true))
  (:Released
    (Variables|Default|SetCanRotate false)))

(event Input|MouseEvents|MouseWheelUp
  (params (Key :type Key%20Structure :default "None"))
  (bind _returnvalue (Game|GetPlayerCameraManager 0))
  (:Pressed
    (bind _output_get (Variables|Default|SetZoomLevel (Math|Integer|Clamp(Integer) (+ (Variables|Default|GetZoomLevel) 1) 1 20)))
    (if (< _output_get 20)
      (Transformation|SetActorLocation (+ (Camera|GetCameraLocation _returnvalue) (* (Math|Vector|GetForwardVector (Camera|GetCameraRotation _returnvalue)) (* (Variables|Default|GetZoomLevel) 5.0))) false false))))

(event Input|MouseEvents|MouseWheelDown
  (params (Key :type Key%20Structure :default "None"))
  (bind _returnvalue (Game|GetPlayerCameraManager 0))
  (:Pressed
    (bind _output_get (Variables|Default|SetZoomLevel (Math|Integer|Clamp(Integer) (+ (Variables|Default|GetZoomLevel) -1) 1 20)))
    (if (> (Math|Conversions|ToByte(Integer) _output_get) 1)
      (Transformation|SetActorLocation (+ (Camera|GetCameraLocation _returnvalue) (* (Math|Vector|GetForwardVector (Camera|GetCameraRotation _returnvalue)) (* (Variables|Default|GetZoomLevel) 5.0))) false false))))

(fn ConstructionScript
  (bind _arrow (Variables|Default|GetArrow))
  (Transformation|SetRelativeRotation _arrow (Math|Rotator|FindLookatRotation (Variables|/Script/Engine.SceneComponent|GetRelativeLocation _arrow) (Math|Vector|Normalize (Variables|Default|GetInspectionVector))) false false)
  (Variables|Default|SetInspectionVector (Math|Vector|Normalize (Variables|Default|GetInspectionVector))))

(fn ToggleDOF
  (params (Enable/Disable :type Boolean))
  (bind _postprocess_volume (Variables|Default|GetPostprocess%20Volume))
  (if Enable/Disable
    (bind _structout (Utilities|Struct|SetmembersinPostProcessSettings (Variables|/Script/Engine.PostProcessVolume|GetSettings _postprocess_volume) 1.1e+02 0.03 1e+02))
    (Variables|/Script/Engine.PostProcessVolume|SetSettings _postprocess_volume _structout)
    (else
      (bind _structout_2 (Utilities|Struct|SetmembersinPostProcessSettings (Variables|/Script/Engine.PostProcessVolume|GetSettings _postprocess_volume) 0.0))
      (Variables|/Script/Engine.PostProcessVolume|SetSettings _postprocess_volume _structout_2))))